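; MovingPlatform is an actor that moves between an initial location and a point on its spline.
; The construction script sets the InterpToMovement component's two relative control points from InitialLocation and the local position of spline point 1.
; It also copies the Duration variable to the component, leaving the movement to InterpToMovement with no event graph logic.
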(event EventBeginPlay)

(event Collision|EventActorBeginOverlap
  (params (OtherActor :type Actor%20Object%20Reference)))

(event EventTick
  (params (DeltaSeconds :type Float%20%28single-precision%29)))

(fn ConstructionScript
  (Variables|/Script/Engine.InterpToMovementComponent|SetControlPoints (Variables|Default|GetInterpToMovement) (Utilities|Array|MakeArray (Utilities|Struct|MakeInterpControlPoint (Variables|Default|GetInitialLocation) true) (Utilities|Struct|MakeInterpControlPoint (Spline|GetLocationatSplinePoint (Variables|Default|GetSpline) 1 "Local") true)))
  (Variables|/Script/Engine.InterpToMovementComponent|SetDuration (Variables|Default|GetInterpToMovement) (Variables|Default|GetDuration)))