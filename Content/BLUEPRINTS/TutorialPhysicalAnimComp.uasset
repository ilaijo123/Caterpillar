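; Tutorial actor component that sets up physical animation on a Caterpillar character's skeletal mesh.
; On BeginPlay it adds a PhysicalAnimationComponent to its owner, casts the owner to Caterpillar, and binds and caches that mesh.
; TogglePhysicalAnimation only switches simulation on for bodies below Spine1, excluding that bone.
; No physical animation settings or profile are applied here, and nothing switches simulation off.
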(event Custom|TogglePhysicalAnimation
  (Class|SkeletalMeshComponent|SetAllBodiesBelowSimulatePhysics (Variables|Default|GetMesh) (Utilities|Name|MakeLiteralName "Spine1") true false))

(event EventBeginPlay
  (bind _returnvalue (Game|AddComponentbyClass (Components|GetOwner) "/Script/Engine.PhysicalAnimationComponent"))
  (bind _output_get (Variables|Default|SetPhysicalAnimationComponent _returnvalue))
  (bind _ascaterpillar (Utilities|Casting|CastToCaterpillar (Components|GetOwner)))
  (Class|PhysicalAnimationComponent|SetSkeletalMeshComponent _output_get (Variables|/Script/Engine.Character|GetMesh _ascaterpillar))
  (Variables|Default|SetMesh (Variables|/Script/Engine.Character|GetMesh _ascaterpillar)))

(event EventTick
  (params (DeltaSeconds :type Float%20%28single-precision%29)))